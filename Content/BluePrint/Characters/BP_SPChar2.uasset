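; BP_SPChar2 is a character Blueprint that configures its appearance and movement speed from data at BeginPlay.
; It looks up the row matching CharName in the SPCharConfig data table and asynchronously loads that row's skeletal mesh asset.
; Once loading completes, it applies the mesh and sets the CharacterMovement max walk speed from the row's attributes.
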(event EventBeginPlay
  (bind _returnvalue (Utilities|GetDataTableRow (Variables|Default|GetSPCharConfig) (Variables|Default|GetCharName))
    (:then
      (Utilities|AsyncLoadAsset (.CharSkeletalMesh (Utilities|Struct|BreakSPCharVisuals (.Visuals (Utilities|Struct|BreakSPCharFullConfig _returnvalue))))
        (:Completed
          (Components|SkeletalMesh|SetSkeletalMeshAsset (Variables|Character|GetMesh) (Utilities|ResolveSoftReference (.CharSkeletalMesh (Utilities|Struct|BreakSPCharVisuals (.Visuals (Utilities|Struct|BreakSPCharFullConfig _returnvalue))))))
          (Variables|/Script/Engine.CharacterMovementComponent|SetMaxWalkSpeed (Variables|Character|GetCharacterMovement) (.MovementSpeed (Utilities|Struct|BreakSpCharAttributes (.Attributes (Utilities|Struct|BreakSPCharFullConfig _returnvalue))))))))))

(fn ConstructionScript)